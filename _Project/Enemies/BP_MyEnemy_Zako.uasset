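; Basic "Zako" enemy character that wanders and takes damage.
; On BeginPlay it requests an AI move to a random reachable nearby point, re-requesting every second without waiting for arrival.
; It also sets IsBattle on its ABP_EnemyZako anim instance, false only in Map_Start, and routes AnyDamage to TakeZakoDamage.
; ExecuteAILogic plays a montage, but its looping timer is disconnected.
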(event `self.ReceiveBeginPlay`
  (bind _returnvalue (`SkeletalMeshComponent.GetAnimInstance` (`self.Mesh`)))
  (`|ExecutionSequence`
    (:`then_0`
      ; Move -Zako
      (`|AIMoveTo` self (`NavigationSystemV1.K2_GetRandomReachablePointInRadius` (`self.K2_GetActorLocation`) 1000.0 null null) null 100.0 :!label _label
        (:`then`
          (`KismetSystemLibrary.Delay` 1.0)
          (goto _label))))
    (:`then_1`
      (bind _returnvalue_2 (`GameplayStatics.GetCurrentLevelName` true))
      (if (`KismetStringLibrary.EqualEqual_StrStr` _returnvalue_2 "Map_Start")
        (bind _asabp_enemy_zako (cast `/Game/_Project/Enemies/ABP_EnemyZako` _returnvalue))
        (set `/Game/_Project/Enemies/ABP_EnemyZako.bIsBattle` false _asabp_enemy_zako)
        (else
          (bind _asabp_enemy_zako_2 (cast `/Game/_Project/Enemies/ABP_EnemyZako` _returnvalue))
          (set `/Game/_Project/Enemies/ABP_EnemyZako.bIsBattle` true _asabp_enemy_zako_2))))))

(event `self.ReceiveAnyDamage`
  (params (Damage :type "Float (single-precision)") (DamageType :type "DamageType Object Reference") (InstigatedBy :type "Controller Object Reference") (DamageCauser :type "Actor Object Reference"))
  (`self.TakeZakoDamage` Damage))

(event `/Game/_Project/Blueprints/BPI_BattleAI.ExecuteAI_Logic`
  ; Motion
  (`self.PlayAnimMontage` "/Game/_Project/Enemies/AM_MyEnemy_Zako.AM_MyEnemy_Zako"))

(fn `UserConstructionScript`)