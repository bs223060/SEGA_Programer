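; Boss enemy that takes damage, attacks through montages, and stays dead via an IsBossDead flag in MyGameInstance.
; AnyDamage lowers HP, prints a one-time rage message at low health, and on death sets that flag and destroys the actor.
; BeginPlay removes an already-defeated boss and starts a looping timer that plays a normal attack, or charge then heavy attack at low HP.
; The BattleTrigger overlap is empty; its L_Battle transition logic is disconnected.
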(event `self.BattleTrigger.OnComponentBeginOverlap`
  (params (OverlappedComponent :type "PrimitiveComponent Object Reference") (OtherActor :type "Actor Object Reference") (OtherComp :type "PrimitiveComponent Object Reference") (OtherBodyIndex :type Integer) (bFromSweep :type Boolean) (SweepResult :type "HitResult Structure (by ref)"))
  ; Change -L_Battle
)

(event `self.ReceiveAnyDamage`
  (params (Damage :type "Float (single-precision)") (DamageType :type "DamageType Object Reference") (InstigatedBy :type "Controller Object Reference") (DamageCauser :type "Actor Object Reference"))
  ; Boss HP
  (`/Engine/EditorBlueprintResources/StandardMacros.IsValid` "BP_BossEnemy"
    (:`Is Valid`
      (bind _output_get (set `self.CurrentHP` (- (`self.CurrentHP`) Damage)))
      (if (> _output_get 0.0)
        (`self.CheckHealthStatus`)
        (if (<= _output_get 80.0)
          (`/Engine/EditorBlueprintResources/StandardMacros.DoOnce` false
            (:`Completed`
              (`KismetSystemLibrary.PrintString` "Angry!!"))))
        (else
          (`/Engine/EditorBlueprintResources/StandardMacros.DoOnce` false
            (:`Completed`
              (bind _asmy_game_instance (cast `MyGameInstance` (`GameplayStatics.GetGameInstance`)))
              (set `MyGameInstance.bIsBossDead` true _asmy_game_instance)
              (`self.K2_DestroyActor`))))))))

(event `self.ReceiveBeginPlay`
  (`|ExecutionSequence`
    (:`then_0`
      ; Display -Boss
      (bind _asmy_game_instance (cast `MyGameInstance` (`GameplayStatics.GetGameInstance`)))
      (if (`MyGameInstance.bIsBossDead` _asmy_game_instance)
        (`self.K2_DestroyActor`)))
    (:`then_1`
      ; Motion
      (`KismetSystemLibrary.K2_SetTimerDelegate` (delegate `BossAI_Logic`) 2.0 true))))

(event `BossAI_Logic`
  ; Motion
  (if (<= (`self.CurrentHP`) 80.0)
    (`self.PlayAnimMontage` "/Game/_Project/Enemies/AM_Boss_Charge.AM_Boss_Charge")
    (`KismetSystemLibrary.Delay` 1.0)
    (`self.PlayAnimMontage` "/Game/_Project/Enemies/AM_Boss_Attack_Heavy.AM_Boss_Attack_Heavy")
    (else
      (`self.PlayAnimMontage` "/Game/_Project/Enemies/AM_Boss_Attack_Normal.AM_Boss_Attack_Normal"))))

(fn `UserConstructionScript`)